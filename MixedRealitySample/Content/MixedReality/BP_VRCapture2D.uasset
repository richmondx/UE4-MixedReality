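; Mixed-reality capture camera actor that registers the render targets of two 2D capture components on BeginPlay and removes them on destruction.
; When FollowController is set, Tick moves it to the tracked left-hand pose of controller index 1, composed with the player's view target transform.
; It then writes its distance to the first DistanceACtor found into a material parameter collection as SearchDepth, and prints that value for debugging.
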(event `self.ReceiveDestroyed`
  (`parent.ReceiveDestroyed`)
  (`SteamVRFunctionLibrary.RemoveCaptureRenderTarget` (`SceneCaptureComponent2D.TextureTarget` (`self.CaptureComponent2D`)) (`SceneCaptureComponent2D.TextureTarget` (`self.SceneCaptureComponent2D`))))

(event `self.ReceiveBeginPlay`
  (`parent.ReceiveBeginPlay`)
  (`SteamVRFunctionLibrary.SetCaptureRenderTarget` (`SceneCaptureComponent2D.TextureTarget` (`self.CaptureComponent2D`)) (`SceneCaptureComponent2D.TextureTarget` (`self.SceneCaptureComponent2D`)))
  (bind _outactors (`GameplayStatics.GetAllActorsOfClass` "/Game/MixedReality/DistanceACtor.DistanceACtor_C"))
  (set `self.DisActor` (`KismetArrayLibrary.Array_Get` _outactors)))

(event `self.ReceiveTick`
  (params (DeltaSeconds :type "Float (single-precision)"))
  (bind (_outposition _outorientation _returnvalue) (`SteamVRFunctionLibrary.GetHandPositionAndOrientation` 1 "Left"))
  (bind _returnvalue_2 (`KismetMathLibrary.VSize` (- (`self.K2_GetActorLocation` (`self.DisActor`)) (`self.K2_GetActorLocation` self))))
  (if (and (`self.FollowController`) _returnvalue)
    (`self.K2_SetActorLocationAndRotation` (`KismetMathLibrary.MakeVector` (.x (.location (`KismetMathLibrary.ComposeTransforms` (`KismetMathLibrary.MakeTransform` _outposition _outorientation) (`self.GetTransform` (`Controller.GetViewTarget` (`GameplayStatics.GetPlayerController` 0)))))) (.y (.location (`KismetMathLibrary.ComposeTransforms` (`KismetMathLibrary.MakeTransform` _outposition _outorientation) (`self.GetTransform` (`Controller.GetViewTarget` (`GameplayStatics.GetPlayerController` 0)))))) (.z (.location (`KismetMathLibrary.ComposeTransforms` (`KismetMathLibrary.MakeTransform` _outposition _outorientation) (`self.GetTransform` (`Controller.GetViewTarget` (`GameplayStatics.GetPlayerController` 0))))))) (.rotation (`KismetMathLibrary.ComposeTransforms` (`KismetMathLibrary.MakeTransform` _outposition _outorientation) (`self.GetTransform` (`Controller.GetViewTarget` (`GameplayStatics.GetPlayerController` 0))))))
    (`KismetMaterialLibrary.SetScalarParameterValue` "/Game/MixedReality/MPC_.MPC_" "SearchDepth" _returnvalue_2)
    (`KismetSystemLibrary.PrintString` (`KismetStringLibrary.Conv_DoubleToString` _returnvalue_2))))

(fn `UserConstructionScript`)